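; Blueprint helper function that returns the number of decimal digits in an integer, named for Int64 values.
; It repeatedly divides the value by 10 inside a bounded loop, counting passes and returning the count once the value drops below 1.
; Zero and any negative input exit on the first pass, so negative numbers do not get their true length.
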(fn GetNumberLength
  (params (Int :type Integer64))
  (LocalVariables|SetNumber Int)
  (for _index (range 0 30)
    (Math|Integer|IncrementInt (LocalVariables|Getj)
      (:%20%20
        (bind _output_get (LocalVariables|SetNumber (/ (LocalVariables|GetNumber) 10)))
        (if (< _output_get 1)
          (return (LocalVariables|Getj)))))))