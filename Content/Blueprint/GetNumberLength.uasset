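; Get Number Length is a utility function that, by its name, is meant to return the digit count of an integer.
; A bounded loop increments a counter, reduces the value modulo 10 and returns the counter once the value is below 1.
; Because it uses modulo instead of division, the value stops changing after the first pass, so the result is not a true digit count.
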(fn GetNumberLength
  (params (Int :type Integer))
  (LocalVariables|SetNumber Int)
  (for _index (range 0 30)
    (Math|Integer|IncrementInt (LocalVariables|Getj)
      (:%20%20
        (bind _output_get (LocalVariables|SetNumber (Math|Integer|%(Integer) (LocalVariables|GetNumber) 10)))
        (if (< _output_get 1)
          (return (LocalVariables|Getj)))))))